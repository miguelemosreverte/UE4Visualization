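; Player character Blueprint that shows timeline element pages in an in-game web browser.
; BeginPlay creates a Browser widget and adds it to the viewport.
; ChangeURL loads a localhost page for the given RowID, shows the widget, then calls RotatePlayerToTheRight.
; That function builds control rotation from forward-vector components rather than current angles, so yaw lands near a fixed 20 degrees instead of turning relatively.
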(event `self.ReceiveBeginPlay`
  (bind _returnvalue (`|CreateWidget` "/Game/Blueprints/Browser.Browser_C" (`GameplayStatics.GetPlayerController` 0)))
  (`UserWidget.AddToViewport` _returnvalue 0)
  (set `self.MyBrowser` _returnvalue))

(event `self.ChangeURL`
  (params (RowID :type Integer))
  (bind _mybrowser (`self.MyBrowser`))
  (`WebBrowser.LoadURL` (`/Game/Blueprints/Browser.WebBrowser_25` _mybrowser) (`KismetStringLibrary.Concat_StrStr` "http://127.0.0.1:8030/p?timelineElementID=" (`KismetStringLibrary.Conv_IntToString` RowID)))
  (`/Game/Blueprints/Browser.Show` _mybrowser)
  (`self.RotatePlayerToTheRight`))

(fn `UserConstructionScript`)