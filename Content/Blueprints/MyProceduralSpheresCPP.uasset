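; Library display actor that builds stacked, labeled rows and spawns a book actor for each data point passed to Render.
; Render clears tracked actors, then places books by vector, scaling Y by a length measured from row bounds.
; Overlap toggles player input for mouse-wheel vertical scrolling; MoveSphereRow forwards row moves.
; The book ID, tracking and sentence-shape steps are disconnected, so new books escape clearing, scrolling and moves.
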(event `self.Box.OnComponentBeginOverlap`
  (params (OverlappedComponent :type "PrimitiveComponent Object Reference") (OtherActor :type "Actor Object Reference") (OtherComp :type "PrimitiveComponent Object Reference") (OtherBodyIndex :type Integer) (bFromSweep :type Boolean) (SweepResult :type "HitResult Structure (by ref)"))
  (`self.EnableInput` (`GameplayStatics.GetPlayerController` 0)))

(event `Key|MouseScrollDown`
  (params (Key :type "Key Structure" :default "AnyKey"))
  (:`Pressed`
    (`self.ScrollLibrary` (* (`self.scrollValue`) -1))))

(event `self.ReceiveActorEndOverlap`
  (params (OtherActor :type "Actor Object Reference"))
  (`self.DisableInput` (`GameplayStatics.GetPlayerController` 0)))

(event `Key|MouseScrollUp`
  (params (Key :type "Key Structure" :default "AnyKey"))
  (:`Pressed`
    (`self.ScrollLibrary` (`self.scrollValue`))))

(event `self.MoveSphereRow`
  (params (RowID :type Integer))
  (for _array_element (`self.LibraryRows`)
    (`LibraryRow.maybeMove` _array_element RowID))
  (for _array_element_2 (`self.Spheres`)
    (`PaulasSphere.maybeMove` _array_element_2 RowID)))

(fn `Render`
  (params (Data :type "Array of Vector Structure") (MaxY :type Integer) (GroupNames :type "Array of String") (ClickOrSentence :type "Array of Boolean") (EventContents :type "Array of String"))
  (bind _libraryrows (`self.LibraryRows`))
  (bind _spheres (`self.Spheres`))
  (bind _currentarrayindex (`self.currentArrayIndex`))
  (for _array_element _spheres
    (`self.K2_DestroyActor` _array_element))
  (`KismetArrayLibrary.Array_Clear` _spheres)
  (for _array_element_2 _libraryrows
    (`self.K2_DestroyActor` _array_element_2))
  (`KismetArrayLibrary.Array_Clear` _libraryrows)
  (for (_array_element_3 _array_index) Data
    (set `self.currentArrayIndex` _array_index)
    (if (< _array_index MaxY)
      (`self.RenderLibraryRow` (`self.currentArrayIndex`) (`KismetArrayLibrary.Array_Get` GroupNames _currentarrayindex)))
    (`self.RenderSphere` _array_element_3 (not (`KismetArrayLibrary.Array_Get` ClickOrSentence _currentarrayindex))))
  (return))

(fn `RenderLibraryRow`
  (params (NewId :type Integer) (GroupName :type String))
  (bind _returnvalue (`|SpawnActorFromClass` "/Game/Blueprints/MyLibraryRowBP.MyLibraryRowBP_C" (`KismetMathLibrary.MakeTransform` (+ (.location (`self.GetTransform`)) (`KismetMathLibrary.MakeVector` 0.0 0.0 (* NewId 20.0))) (.rotation (`self.GetTransform`)) (.scale (`self.GetTransform`))) "Undefined" "OverrideRootScale"))
  (`TextRenderComponent.K2_SetText` (`/Game/Blueprints/MyLibraryRowBP.TextRender4` _returnvalue) (`KismetTextLibrary.Conv_StringToText` GroupName))
  (`LibraryRow.setID` _returnvalue NewId)
  (`self.SetLibraryLength` _returnvalue)
  (`KismetArrayLibrary.Array_Add` (`self.LibraryRows`) _returnvalue)
  (return))

(fn `RenderSphere`
  (params (InVec :type "Vector Structure") (IsSentence :type Boolean))
  (bind _returnvalue (+ (.location (`self.GetTransform`)) (`KismetMathLibrary.MakeVector` (.x InVec) (- (* (.y InVec) (`self.LibraryLength`)) (`self.HalfLibraryLength`)) (.z InVec))))
  (bind _returnvalue_2 (`|SpawnActorFromClass` "/Game/Books/NEW_book.NEW_book_C" (`KismetMathLibrary.MakeTransform` _returnvalue (.rotation (`self.GetTransform`)) (.scale (`self.GetTransform`))) "AlwaysSpawn" "OverrideRootScale" null false true))
  (`self.K2_SetActorRelativeTransform` _returnvalue_2 (`KismetMathLibrary.MakeTransform` (`KismetMathLibrary.MakeVector` (+ (.x _returnvalue) 25.0) (.y _returnvalue) (+ (.z _returnvalue) 40.0)) (struct :`Yaw` -179.899994 :`Roll` 90.0) (0.4 0.4 0.4)) false false))

(fn `setLibraryLength`
  (params (NewParam :type "Actor Object Reference"))
  (if (== (`self.LibraryLength`) 0.0)
    (bind _output_get (set `self.LibraryLength` (.y (`.BoxExtent` (`self.GetActorBounds` NewParam false)))))
    (set `self.HalfLibraryLength` (/ _output_get 2.0))))

(fn `UserConstructionScript`)